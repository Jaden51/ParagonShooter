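; BP_KillAllGameMode is a game mode that spawns the player's chosen character class when play begins.
; On BeginPlay it loops over every PlayerStart, reads the class from BP_GameInstance and passes it with that start's transform to player 0's BP_ShooterController.SpawnCharacter.
; The spawn call runs once per PlayerStart, and the graph holds no kill-all or win-condition logic.
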(event `self.ReceiveBeginPlay`
  (bind _outactors (`GameplayStatics.GetAllActorsOfClass` "/Script/Engine.PlayerStart"))
  (for _array_element _outactors
    (set `self.SpawnTransform` (`self.GetTransform` _array_element))
    (bind _asbp_game_instance (cast `/Game/GameModes/BP_GameInstance` (`GameplayStatics.GetGameInstance`)))
    (bind _output_get (set `self.GameInstance` _asbp_game_instance))
    (bind _class (`/Game/GameModes/BP_GameInstance.GetPlayerClass` _output_get))
    (set `self.ClassToSpawn` _class)
    (bind _asbp_shooter_controller (cast `/Game/Characters/BP_ShooterController` (`GameplayStatics.GetPlayerController` 0)))
    (`/Game/Characters/BP_ShooterController.SpawnCharacter` _asbp_shooter_controller (`self.ClassToSpawn`) (`self.SpawnTransform`))))

(fn `UserConstructionScript`)